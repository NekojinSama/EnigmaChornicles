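; StartTimer_2 is a trigger actor that runs an on-screen minutes and seconds timer for the third-person character.
; BeginPlay creates the ScreenTimer widget, which Box overlap adds to the viewport while enabling this actor's Tick.
; A one-second tick interval, set on all StartTimer_2 instances, turns Tick into the counter.
; EndBox overlap disables Tick on all instances, and each box destroys itself after use.
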(event `self.ReceiveTick`
  (params (DeltaSeconds :type "Float (single-precision)"))
  (set `self.TimerSeconds` (+ (`self.TimerSeconds`) 1))
  (if (> (`self.TimerSeconds`) 59)
    (set `self.TimerMinutes` (+ (`self.TimerMinutes`) 1))
    (set `self.TimerSeconds` 0)))

(event `self.ReceiveBeginPlay`
  (bind _outactors (`GameplayStatics.GetAllActorsOfClass` "StartTimer_2_C"))
  (bind _returnvalue (`|CreateWidget` "/Game/UI/ScreenTimer.ScreenTimer_C"))
  (set `self.TimerUI` _returnvalue))

(event `self.Box.OnComponentBeginOverlap`
  (params (OverlappedComponent :type "PrimitiveComponent Object Reference") (OtherActor :type "Actor Object Reference") (OtherComp :type "PrimitiveComponent Object Reference") (OtherBodyIndex :type Integer) (bFromSweep :type Boolean) (SweepResult :type "HitResult Structure (by ref)"))
  (cast `/Game/ThirdPerson/Blueprints/BP_ThirdPersonCharacter` OtherActor)
  (`UserWidget.AddToViewport` (`self.TimerUI`) 0)
  (`self.SetActorTickInterval` (stale `self.ReceiveBeginPlay` _outactors) 1.0)
  (`self.SetActorTickEnabled` true)
  (`ActorComponent.K2_DestroyComponent` (`self.Box`)))

(event `self.EndBox.OnComponentBeginOverlap`
  (params (OverlappedComponent :type "PrimitiveComponent Object Reference") (OtherActor :type "Actor Object Reference") (OtherComp :type "PrimitiveComponent Object Reference") (OtherBodyIndex :type Integer) (bFromSweep :type Boolean) (SweepResult :type "HitResult Structure (by ref)"))
  (cast `/Game/ThirdPerson/Blueprints/BP_ThirdPersonCharacter` OtherActor)
  (`self.SetActorTickEnabled` (stale `self.ReceiveBeginPlay` _outactors) false)
  (`ActorComponent.K2_DestroyComponent` (`self.EndBox`)))

(fn `UserConstructionScript`)