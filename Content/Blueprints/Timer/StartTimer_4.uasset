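; StartTimer_4 is a trigger-driven stopwatch that times the player between a start box and an end box.
; BeginPlay creates a ScreenTimer_2 widget and moves EndBox to EndLocation.
; When BP_ThirdPersonCharacter enters Box, the widget appears and a one-second timer, looping per TimerBool, counts seconds and minutes.
; Entering EndBox clears that timer, and each box destroys itself after the character triggers it.
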(event `self.ReceiveTick`
  (params (DeltaSeconds :type "Float (single-precision)")))

(event `StartTimerEvent`
  (set `self.TimerSeconds` (+ (`self.TimerSeconds`) 1))
  (if (> (`self.TimerSeconds`) 59)
    (set `self.TimerMinutes` (+ (`self.TimerMinutes`) 1))
    (set `self.TimerSeconds` 0)))

(event `self.ReceiveBeginPlay`
  (bind _returnvalue (`|CreateWidget` "/Game/UI/TimerUI/ScreenTimer_2.ScreenTimer_2_C" (`GameplayStatics.GetPlayerController` 0)))
  (set `self.TimerWidget` _returnvalue)
  (`SceneComponent.K2_SetWorldLocation` (`self.EndBox`) (`self.EndLocation`) false true))

(event `self.Box.OnComponentBeginOverlap`
  (params (OverlappedComponent :type "PrimitiveComponent Object Reference") (OtherActor :type "Actor Object Reference") (OtherComp :type "PrimitiveComponent Object Reference") (OtherBodyIndex :type Integer) (bFromSweep :type Boolean) (SweepResult :type "HitResult Structure (by ref)"))
  (bind _returnvalue (`GameplayStatics.GetPlayerController` 0))
  (bind _timerwidget (`self.TimerWidget`))
  (cast `/Game/ThirdPerson/Blueprints/BP_ThirdPersonCharacter` OtherActor)
  (`UserWidget.AddToViewport` _timerwidget 0)
  (`WidgetBlueprintLibrary.SetInputMode_GameAndUIEx` (`GameplayStatics.GetPlayerController` 0) _timerwidget)
  (set `PlayerController.bShowMouseCursor` false _returnvalue)
  (`WidgetBlueprintLibrary.SetInputMode_GameOnly` _returnvalue)
  (bind _returnvalue_2 (`KismetSystemLibrary.K2_SetTimerDelegate` (delegate `StartTimerEvent`) 1.0 (`self.TimerBool`)))
  (`ActorComponent.K2_DestroyComponent` (`self.Box`)))

(event `self.EndBox.OnComponentBeginOverlap`
  (params (OverlappedComponent :type "PrimitiveComponent Object Reference") (OtherActor :type "Actor Object Reference") (OtherComp :type "PrimitiveComponent Object Reference") (OtherBodyIndex :type Integer) (bFromSweep :type Boolean) (SweepResult :type "HitResult Structure (by ref)"))
  (cast `/Game/ThirdPerson/Blueprints/BP_ThirdPersonCharacter` OtherActor)
  (`KismetSystemLibrary.K2_ClearAndInvalidateTimerHandle` (stale `self.Box.OnComponentBeginOverlap` _returnvalue_2))
  (`ActorComponent.K2_DestroyComponent` (`self.EndBox`)))

(fn `UserConstructionScript`)