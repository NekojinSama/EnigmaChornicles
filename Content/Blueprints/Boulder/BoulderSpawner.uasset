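; Actor that repeatedly spawns Boulder actors at its own transform and launches them.
; On BeginPlay it calls BoulderForceLife once, then repeats it on a looping timer set by ObjectSpawnTimer.
; Each call pushes the new boulder's static mesh with an AddForce impulse as a velocity change, so mass is ignored, and gives it a lifespan from ObjectLifeSpan so old boulders clean themselves up.
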(event `self.ReceiveBeginPlay`
  (`self.BoulderForceLife`)
  (`KismetSystemLibrary.K2_SetTimer` null "BoulderForceLife" (`self.ObjectSpawnTimer`) true))

(fn `BoulderForceLife`
  (bind _returnvalue (`|SpawnActorFromClass` "/Game/Blueprints/Boulder/Boulder.Boulder_C" (`self.GetTransform`) "Undefined" "OverrideRootScale" null null))
  (`PrimitiveComponent.AddImpulse` (`/Game/Blueprints/Boulder/Boulder.StaticMesh` _returnvalue) (`self.AddForce`) "None" true)
  (`self.SetLifeSpan` _returnvalue (`self.ObjectLifeSpan`)))

(fn `UserConstructionScript`)