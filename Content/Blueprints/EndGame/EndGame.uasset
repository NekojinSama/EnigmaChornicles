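; EndGame is a trigger actor that ends the game when the player's third-person character enters its EndPromt collision component.
; On BeginPlay it pre-creates a GameEndPromt widget for the first player controller.
; On overlap with BP_ThirdPersonCharacter it pauses the game, adds that widget to the viewport, shows the mouse cursor and switches input to UI-only focused on the widget.
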(event `self.ReceiveBeginPlay`
  (bind _returnvalue (`|CreateWidget` "/Game/UI/GameFinishUI/GameEndPromt.GameEndPromt_C" (`GameplayStatics.GetPlayerController` 0)))
  (set `self.EndGameWidget` _returnvalue))

(event `self.EndPromt.OnComponentBeginOverlap`
  (params (OverlappedComponent :type "PrimitiveComponent Object Reference") (OtherActor :type "Actor Object Reference") (OtherComp :type "PrimitiveComponent Object Reference") (OtherBodyIndex :type Integer) (bFromSweep :type Boolean) (SweepResult :type "HitResult Structure (by ref)"))
  (bind _returnvalue (`GameplayStatics.GetPlayerController` 0))
  (cast `/Game/ThirdPerson/Blueprints/BP_ThirdPersonCharacter` OtherActor)
  (`GameplayStatics.SetGamePaused` true)
  (`UserWidget.AddToViewport` (`self.EndGameWidget`) 0)
  (set `PlayerController.bShowMouseCursor` true _returnvalue)
  (`WidgetBlueprintLibrary.SetInputMode_UIOnlyEx` _returnvalue (`self.EndGameWidget`)))

(fn `UserConstructionScript`)